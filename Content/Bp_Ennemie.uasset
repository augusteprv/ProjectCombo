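; Enemy Blueprint that turns to face the player and plays an attack montage when the player comes within range.
; On BeginPlay and every Tick it sets its yaw toward player 0's location.
; Player overlap with the Sphere starts a one-second attack timer through a DoOnce, which resets when the montage completes.
; End overlap only clears the Looping variable passed at timer creation; the timer itself is never cleared.
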(event `self.ReceiveBeginPlay`
  (bind (_returnvalue_roll _returnvalue_pitch _returnvalue_yaw) (`KismetMathLibrary.BreakRotator` (`KismetMathLibrary.FindLookAtRotation` (`self.K2_GetActorLocation`) (`self.K2_GetActorLocation` (`GameplayStatics.GetPlayerCharacter` 0)))))
  (`self.K2_SetActorRotation` (`KismetMathLibrary.MakeRotator` 0.0 0.0 _returnvalue_yaw) :!label _label))

(event `self.ReceiveTick`
  (params (DeltaSeconds :type "Float (single-precision)"))
  (goto _label))

(event `self.Sphere.OnComponentBeginOverlap`
  (params (OverlappedComponent :type "PrimitiveComponent Object Reference") (OtherActor :type "Actor Object Reference") (OtherComp :type "PrimitiveComponent Object Reference") (OtherBodyIndex :type Integer) (bFromSweep :type Boolean) (SweepResult :type "HitResult Structure (by ref)"))
  (if (== OtherActor (`GameplayStatics.GetPlayerCharacter` 0))
    (`/Engine/EditorBlueprintResources/StandardMacros.DoOnce` false :!label _label_2
      (:`Completed`
        (`KismetSystemLibrary.K2_SetTimerDelegate` (delegate `Attack_Ennemie_anim`) 1.0 (`self.Looping`))))))

(event `Attack_Ennemie_anim`
  (`|PlayMontage` (`self.SkeletalMesh`) "/Game/Sword_Animations/Animations/Sequence1/02_Attack/03_Combo_Attack_03/Combo_Attack_03_01_Seq_Montage.Combo_Attack_03_01_Seq_Montage"
    (:`OnCompleted`
      (goto _label_2 :!via `Reset`))))

(event `self.Sphere.OnComponentEndOverlap`
  (params (OverlappedComponent :type "PrimitiveComponent Object Reference") (OtherActor :type "Actor Object Reference") (OtherComp :type "PrimitiveComponent Object Reference") (OtherBodyIndex :type Integer))
  (set `self.Looping` false))

(fn `UserConstructionScript`)